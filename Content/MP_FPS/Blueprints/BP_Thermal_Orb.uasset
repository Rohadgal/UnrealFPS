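; BP_Thermal_Orb is a pickup that gives an overlapping BP_Character_Master temporary thermal vision.
; On overlap it calls SetThermalVision, toggles its mesh visibility, disables sphere collision and plays a pickup sound at world origin.
; After a delay read from the character's ThermalVisionTimer, it restores the orb and turns the effect off through ServerToggleThermalVision, unlike the direct call that enables it.
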(event Collision|EventActorBeginOverlap
  (params (OtherActor :type Actor%20Object%20Reference))
  (bind _asbp_character_master (Utilities|Casting|CastToBP_Character_Master OtherActor))
  (Utilities|IsValid _asbp_character_master
    (:Is%20Valid
      (Default|SetThermalVision _asbp_character_master true)
      (Rendering|ToggleVisibility (Variables|Default|GetStaticMesh) false)
      (Collision|SetCollisionEnabled (Variables|Default|GetSphere) "NoCollision")
      (Audio|PlaySoundatLocation "/Game/MP_FPS/MilitaryWeapSilver/Sound/GrenadeLauncher/Cues/GrenadeLauncher_AmmoPickup_Cue.GrenadeLauncher_AmmoPickup_Cue" "0, 0, 0")
      (Utilities|FlowControl|Delay (Variables|/Game/MP_FPS/Characters/Blueprints/BP_Character_Master.BP_Character_Master_C|GetThermalVisionTimer _asbp_character_master))
      (Rendering|ToggleVisibility (Variables|Default|GetStaticMesh) true)
      (Collision|SetCollisionEnabled (Variables|Default|GetSphere) "QueryAndPhysics")
      (Utilities|IsValid _asbp_character_master
        (:Is%20Valid
          (Default|ServerToggleThermalVision _asbp_character_master false))))))

(fn ConstructionScript)