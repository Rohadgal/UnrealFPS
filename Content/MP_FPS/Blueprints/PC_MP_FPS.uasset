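; PC_MP_FPS is the multiplayer FPS player controller, handling team choice and respawn requests.
; Server_SetPCTeam stores the Team, which Server_RequestRespawn passes to GM_MP_FPS along with the controller so the game mode respawns the player.
; Pressing Tab creates the BPW_TeamSelect widget with its resume button enabled, then switches to UI-only input with a visible cursor.
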(event Custom|Server_RequestRespawn
  (bind _returnvalue (Game|GetGameMode))
  (Utilities|IsValid _returnvalue
    (:Is%20Valid
      (bind _asgm_mp_fps (Utilities|Casting|CastToGM_MP_FPS _returnvalue))
      (Utilities|IsValid _asgm_mp_fps
        (:Is%20Valid
          (Default|ServerRespawnPlayer _asgm_mp_fps self (Variables|Default|GetTeam)))))))

(event Custom|Server_SetPCTeam
  (params (Team :type E_Teams%20Enum))
  (Variables|Default|SetTeam Team))

(event Input|KeyboardEvents|Tab
  (params (Key :type Key%20Structure :default "AnyKey"))
  (bind _self self)
  (:Pressed
    (bind _returnvalue (UserInterface|CreateWidget "/Game/MP_FPS/Widgets/UI/BPW_TeamSelect.BPW_TeamSelect_C" _self))
    (UserInterface|Viewport|AddtoViewport _returnvalue 0)
    (Widget|SetIsEnabled (Variables|/Game/MP_FPS/Widgets/UI/BPW_TeamSelect.BPW_TeamSelect_C|Getresume_btn _returnvalue) true)
    (Input|SetInputModeUIOnly _self _returnvalue "DoNotLock")
    (Variables|Default|SetbShowMouseCursor true)))

(fn ConstructionScript)