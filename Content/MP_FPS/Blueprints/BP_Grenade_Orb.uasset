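; BP_Grenade_Orb is a grenade pickup actor for the multiplayer FPS.
; When a BP_Character_Master overlaps it, it calls ServerSetGrenadeType on that character and plays the grenade launcher ammo pickup sound at the mesh location.
; It hides its mesh and disables sphere collision, then restores both after a short delay so the pickup respawns in place.
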(event Collision|EventActorBeginOverlap
  (params (OtherActor :type Actor%20Object%20Reference))
  (bind _asbp_character_master (Utilities|Casting|CastToBP_Character_Master OtherActor))
  (Utilities|IsValid _asbp_character_master
    (:Is%20Valid
      (bind _output_get (Variables|Default|SetcharacterReference _asbp_character_master))
      (Default|ServerSetGrenadeType _output_get)
      (Rendering|ToggleVisibility (Variables|Default|GetStaticMesh) false)
      (Collision|SetCollisionEnabled (Variables|Default|GetSphere) "NoCollision")
      (Audio|PlaySoundatLocation "/Game/MP_FPS/MilitaryWeapSilver/Sound/GrenadeLauncher/Cues/GrenadeLauncher_AmmoPickup_Cue.GrenadeLauncher_AmmoPickup_Cue" (Transformation|GetWorldLocation (Variables|Default|GetStaticMesh)))
      (Utilities|FlowControl|Delay 5.0)
      (Rendering|ToggleVisibility (Variables|Default|GetStaticMesh) true)
      (Collision|SetCollisionEnabled (Variables|Default|GetSphere) "QueryAndPhysics"))))

(fn ConstructionScript)