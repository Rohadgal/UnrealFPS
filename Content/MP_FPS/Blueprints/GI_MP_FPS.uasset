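; Game instance for the MP_FPS game that handles menu display and the start of single-player and multiplayer games.
; Events create the main, multiplayer and server list widgets, with the main menu also setting UI-only input.
; Single-player and hosting open the same test map with game-only input, hosting first creating a non-LAN session and loading as a listen server.
; Joining takes a session search result, and host or join failures only print a message.
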(event Custom|ShowMultiplayerMenu
  (bind _returnvalue (UserInterface|CreateWidget "/Game/MP_FPS/Widgets/UI/BPW_MultiplayerMenu.BPW_MultiplayerMenu_C" (Game|GetPlayerController 0)))
  (bind _output_get (Variables|Default|SetMultiplayerMenu_Ref _returnvalue))
  (UserInterface|Viewport|AddtoViewport _output_get 0))

(event Custom|ShowMainMenu
  (bind _returnvalue (Game|GetPlayerController 0))
  (bind _returnvalue_2 (UserInterface|CreateWidget "/Game/MP_FPS/Widgets/UI/BPW_MainMenu.BPW_MainMenu_C" _returnvalue))
  (bind _output_get (Variables|Default|SetMainMenu_Ref _returnvalue_2))
  (UserInterface|Viewport|AddtoViewport _output_get 0)
  (Input|SetInputModeUIOnly _returnvalue _output_get "DoNotLock")
  (Variables|/Script/Engine.PlayerController|SetbShowMouseCursor _returnvalue true))

(event Custom|ShowServerList
  (bind _returnvalue (UserInterface|CreateWidget "/Game/MP_FPS/Widgets/UI/BPW_ServerList.BPW_ServerList_C" (Game|GetPlayerController 0)))
  (bind _output_get (Variables|Default|SetServerList _returnvalue))
  (UserInterface|Viewport|AddtoViewport _output_get 0))

(event Custom|StartSinglePlayer
  (bind _returnvalue (Game|GetPlayerController 0))
  (Game|OpenLevel(byName) "Test_Map_001")
  (Input|SetInputModeGameOnly _returnvalue)
  (Variables|/Script/Engine.PlayerController|SetbShowMouseCursor _returnvalue false))

(event Custom|HostGame
  (bind _returnvalue (Game|GetPlayerController 0))
  (|Session _returnvalue 10 false
    (:OnSuccess
      (Game|OpenLevel(byName) "Test_Map_001" true "listen")
      (Input|SetInputModeGameOnly _returnvalue)
      (Variables|/Script/Engine.PlayerController|SetbShowMouseCursor _returnvalue false))
    (:OnFailure
      (Development|PrintString "Host Game Failed!"))))

(event Custom|JoinSession
  (params (Session :type Blueprint%20Session%20Result%20Structure))
  (|JoinSession (Game|GetPlayerController 0) Session
    (:OnFailure
      (Development|PrintString "Failed To Join Session!!!"))))