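; Master weapon Blueprint for a multiplayer FPS, handling hitscan fire and its effects, with no damage logic yet.
; On fire, the client sphere-traces from the character's camera to find the aim point, then from the first-person muzzle toward it.
; The result passes through a server event to a multicast that plays fire sound and impact effects.
; Muzzle flashes spawn on both meshes, with first-person owner-only and third-person hidden from the owner.
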(event Custom|Client_OnWeaponFire
  (bind _bp_charactermasterref (Variables|Default|GetBP_CharacterMasterRef))
  (bind _array (Utilities|Array|MakeArray _bp_charactermasterref))
  (bind _fp_cam (Variables|/Game/MP_FPS/Characters/Blueprints/BP_Character_Master.BP_Character_Master_C|GetFP_Cam _bp_charactermasterref))
  (bind _returnvalue (Transformation|GetWorldLocation _fp_cam))
  (bind (_outhit _returnvalue_2) (Collision|SphereTraceByChannel _returnvalue (+ _returnvalue (* (Math|Vector|GetForwardVector (Transformation|GetWorldRotation _fp_cam)) 4e+03)) 2.0 "TraceTypeQuery1" false _array "None"))
  (bind (_outhit_2 _returnvalue_3) (Collision|SphereTraceByChannel (Transformation|GetSocketLocation (Variables|Default|GetSK_FP_Weapon) "MuzzleFlash") (Math|Vector|SelectVector (.ImpactPoint (Collision|BreakHitResult _outhit)) (.TraceEnd (Collision|BreakHitResult _outhit)) _returnvalue_2) 2.0 "TraceTypeQuery1" false _array "None"))
  (CallFunction|ServerShootInfo _outhit_2 _returnvalue_3))

(event Custom|Client_OffWeaponFire)

(event Custom|MultiCast_WeaponFX
  (params (HitResult :type Hit%20Result%20Structure) (Hit :type Boolean))
  (bind (_bblockinghit _binitialoverlap _time _location _impactpoint _normal _impactnormal) (Collision|BreakHitResult HitResult))
  (bind _sk_fp_weapon (Variables|Default|GetSK_FP_Weapon))
  (Audio|SpawnSoundAttached "/Game/MP_FPS/MilitaryWeapSilver/Sound/Rifle/Cues/RifleA_Fire_Cue.RifleA_Fire_Cue" _sk_fp_weapon "MuzzleFlash")
  (Utilities|FlowControl|Sequence
    (:then_0
      (bind _returnvalue (Effects|SpawnEmitterAttached "/Game/MP_FPS/MilitaryWeapSilver/FX/P_AssaultRifle_MuzzleFlash.P_AssaultRifle_MuzzleFlash" _sk_fp_weapon "MuzzleFlash" "0, 0, 0" "0, 0, 0" "SnapToTarget"))
      (Rendering|SetOnlyOwnerSee _returnvalue true :!class /Script/Engine.PrimitiveComponent)
      (if Hit
        (Audio|PlaySoundatLocation "/Game/MP_FPS/MilitaryWeapSilver/Sound/Rifle/Cues/Rifle_ImpactSurface_Cue.Rifle_ImpactSurface_Cue" _impactpoint)
        (Effects|SpawnEmitteratLocation "/Game/MP_FPS/MilitaryWeapSilver/FX/P_Impact_Metal_Medium_01.P_Impact_Metal_Medium_01" _impactpoint (Math|Rotator|MakeRotfromZ _impactnormal))))
    (:then_1
      (bind _returnvalue_2 (Effects|SpawnEmitterAttached "/Game/MP_FPS/MilitaryWeapSilver/FX/P_AssaultRifle_MuzzleFlash.P_AssaultRifle_MuzzleFlash" (Variables|Default|GetSK_TP_Weapon) "MuzzleFlash" "0, 0, 0" "0, 0, 0" "SnapToTarget"))
      (Class|PrimitiveComponent|SetOwnerNoSee _returnvalue_2 true))))

(event Custom|Server_ShootInfo
  (params (HitResult :type Hit%20Result%20Structure) (Hit :type Boolean))
  (CallFunction|MultiCastWeaponFX HitResult Hit))

(fn ConstructionScript)