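; BP_Grenade is a thrown or launched grenade actor that detonates on a three-second fuse after BeginPlay, with its mesh ignoring the instigator while moving.
; Detonate switches on GrenadeType, but Flash, Fragment and Slow all share one path: spawn BP_Explosion, play a sound and destroy the grenade.
; Type-specific flash (ClientFlash on overlapping characters) and slow-smoke logic exist but are disconnected.
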(event Custom|Detonate
  (switch Utilities|FlowControl|Switch|SwitchonEnum_GrenadeType (Variables|Default|GetgrenadeType)
    (:NewEnumerator1
      _)
    (:NewEnumerator2
      _)
    (:NewEnumerator3
      _))
  (Game|SpawnActorfromClass "/Game/MP_FPS/Grenades/Explosion/BP_Explosion.BP_Explosion_C" (Transformation|GetActorTransform) "Undefined" 0 0)
  (Audio|PlaySoundatLocation "/Game/MP_FPS/MilitaryWeapSilver/Sound/GrenadeLauncher/Wavs/GrenadeLauncher_Explosion01.GrenadeLauncher_Explosion01" (Transformation|GetActorLocation))
  (Actor|DestroyActor))

(event EventBeginPlay
  (Collision|IgnoreActorwhenMoving (Variables|Default|GetSM_Grenade) (Game|GetInstigator) true)
  (Utilities|FlowControl|Delay 3.0)
  (CallFunction|Detonate))

(fn ConstructionScript)