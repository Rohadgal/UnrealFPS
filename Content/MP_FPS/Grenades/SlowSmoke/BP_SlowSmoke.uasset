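; BP_SlowSmoke is the area effect of a slow-smoke grenade, a temporary sphere that affects player characters inside it.
; On BeginPlay a timeline scales the sphere uniformly, and a 7-second delay started from its update output then destroys the actor.
; Sphere overlap begin and end call the server start and stop slow-smoke events on any overlapping BP_Character_Master.
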(event OnComponentBeginOverlap(SM_Sphere)
  (params (OverlappedComponent :type Primitive%20Component%20Object%20Reference) (OtherActor :type Actor%20Object%20Reference) (OtherComp :type Primitive%20Component%20Object%20Reference) (OtherBodyIndex :type Integer) (bFromSweep :type Boolean) (SweepResult :type Hit%20Result%20Structure%20%28by%20ref%29))
  (bind _asbp_character_master (Utilities|Casting|CastToBP_Character_Master OtherActor))
  (Default|ServerStartSlowSmoke _asbp_character_master))

(event OnComponentEndOverlap(SM_Sphere)
  (params (OverlappedComponent :type Primitive%20Component%20Object%20Reference) (OtherActor :type Actor%20Object%20Reference) (OtherComp :type Primitive%20Component%20Object%20Reference) (OtherBodyIndex :type Integer))
  (bind _asbp_character_master (Utilities|Casting|CastToBP_Character_Master OtherActor))
  (Default|ServerStopSlowSmoke _asbp_character_master))

(event Custom|Update
  (params (scale :type Float%20%28single-precision%29))
  (Transformation|SetWorldScale3D (Variables|Default|GetSM_Sphere) (Math|Vector|MakeVector scale scale scale)))

(event EventBeginPlay
  (bind _scale (Timeline|ScaleTimeline PlayFromStart)
    (:Update
      (CallFunction|Update _scale)
      (Utilities|FlowControl|Delay 7.0)
      (Actor|DestroyActor))))

(fn ConstructionScript)